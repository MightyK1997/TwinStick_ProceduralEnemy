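; Actor Blueprint that textures a stone ground object with a dynamic material at BeginPlay.
; It creates a dynamic instance of a stone material on the ground component's first slot.
; A Sequence then feeds five stone textures into top, right, left, bottom and center texture parameters, which the file name suggests are meant for blending.
; Overlap, Tick and the construction script are empty.
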(event `self.ReceiveBeginPlay`
  (bind _returnvalue (`PrimitiveComponent.CreateDynamicMaterialInstance` (`self.Obj_StoneGround`) 0 (`self.Var_Stone`)))
  (`|ExecutionSequence`
    (:`then_0`
      (`MaterialInstanceDynamic.SetTextureParameterValue` _returnvalue "T_Top" (`self.StoneTop`)))
    (:`then_1`
      (`MaterialInstanceDynamic.SetTextureParameterValue` _returnvalue "T_Right" (`self.StoneRight`)))
    (:`then_2`
      (`MaterialInstanceDynamic.SetTextureParameterValue` _returnvalue "T_Left" (`self.StoneLeft`)))
    (:`then_3`
      (`MaterialInstanceDynamic.SetTextureParameterValue` _returnvalue "T_Bottom" (`self.StoneBottom`)))
    (:`then_4`
      (`MaterialInstanceDynamic.SetTextureParameterValue` _returnvalue "T_Center" (`self.StoneCenter`)))))

(fn `UserConstructionScript`)